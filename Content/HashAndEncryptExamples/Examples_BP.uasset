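; Example actor Blueprint that demonstrates string hashing and custom encryption helper functions through printed output.
; On BeginPlay it prints two near-identical short strings and their hashes.
; Disconnected chains, which never run, wrap a hashed phrase in random strings, encrypt it, round-trip it through bytes and decrypt it.
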(event `self.ReceiveBeginPlay`
  (bind _returnvalue (`KismetStringLibrary.Concat_StrStr` "AC"))
  (bind _returnvalue_2 (`KismetStringLibrary.Concat_StrStr` "AB"))
  (`|ExecutionSequence`
    (:`then_1`
      (`|ExecutionSequence`
        (:`then_0`
          (`KismetSystemLibrary.PrintString` _returnvalue_2 true true (struct :`G` 0.66 :`B` 1.0 :`A` 1.0) 60.0)
          (`KismetSystemLibrary.PrintString` _returnvalue true true (struct :`G` 0.66 :`B` 1.0 :`A` 1.0) 60.0)
          (bind _returnvalue_3 (`HashAndEncryptToolsPluginBPLibrary.ConvertStringToHash` _returnvalue_2))
          (`KismetSystemLibrary.PrintString` _returnvalue_3 true true (struct :`G` 0.66 :`B` 1.0 :`A` 1.0) 60.0)
          (bind _returnvalue_4 (`HashAndEncryptToolsPluginBPLibrary.ConvertStringToHash` _returnvalue))
          (`KismetSystemLibrary.PrintString` _returnvalue_4 true true (struct :`G` 0.66 :`B` 1.0 :`A` 1.0) 60.0))))))

(fn `UserConstructionScript`)